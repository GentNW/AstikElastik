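; BP_Health is a health pack pickup that restores a small amount of the player's health on overlap.
; On BeginPlay it caches the player pawn as BP_ThirdPersonCharacter.
; When that player overlaps it below full health, it adds a fixed increment without clamping, then destroys itself.
; AddHealth also increments the player's HealthPickedUp, then immediately resets it to zero.
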(event EventBeginPlay
  (CallFunction|SetupPlayerInstance))

(event Collision|EventActorBeginOverlap
  (params (OtherActor :type Actor%20Object%20Reference))
  (if (== (Variables|Default|GetPlayer) OtherActor)
    ;[1 1 1] Using the HealthPack
    (if (CallFunction|IsHealthNotFull)
      (CallFunction|AddHealth)
      (Actor|DestroyActor))))

(event EventTick
  (params (DeltaSeconds :type Float%20%28single-precision%29)))

(fn ConstructionScript)

(fn AddHealth
  (bind _player (Variables|Default|GetPlayer))
  (Variables|/Game/ThirdPerson/Blueprints/BP_ThirdPersonCharacter.BP_ThirdPersonCharacter_C|SetHealth _player (+ (Variables|/Game/ThirdPerson/Blueprints/BP_ThirdPersonCharacter.BP_ThirdPersonCharacter_C|GetHealth _player) 0.05))
  (Math|Integer|IncrementInt (Variables|/Game/ThirdPerson/Blueprints/BP_ThirdPersonCharacter.BP_ThirdPersonCharacter_C|GetHealthPickedUp _player)
    (:%20%20
      (Variables|/Game/ThirdPerson/Blueprints/BP_ThirdPersonCharacter.BP_ThirdPersonCharacter_C|SetHealthPickedUp _player 0))))

(fn IsHealthNotFull
  (return (< (Variables|/Game/ThirdPerson/Blueprints/BP_ThirdPersonCharacter.BP_ThirdPersonCharacter_C|GetHealth (Variables|Default|GetPlayer)) 1.0)))

(fn SetupPlayerInstance
  (bind _asbp_third_person_character (Utilities|Casting|CastToBP_ThirdPersonCharacter (Game|Player|GetPlayerPawn 0)))
  (Variables|Default|SetPlayer _asbp_third_person_character))